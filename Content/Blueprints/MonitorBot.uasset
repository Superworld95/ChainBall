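; MonitorBot is an actor that turns to face a character that enters its sphere trigger.
; Sphere overlap stores the character and starts a looping timer that eases the actor's yaw toward it with RInterpTo.
; The end-overlap handler would clear that timer, but its binding never runs, so tracking is not stopped on exit.
; Any overlap with the Box turns on physics simulation for the Body.
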(event OnComponentBeginOverlap(Sphere)
  (params (OverlappedComponent :type Primitive%20Component%20Object%20Reference) (OtherActor :type Actor%20Object%20Reference) (OtherComp :type Primitive%20Component%20Object%20Reference) (OtherBodyIndex :type Integer) (bFromSweep :type Boolean) (SweepResult :type Hit%20Result%20Structure%20%28by%20ref%29))
  (bind _ascharacter (Utilities|Casting|CastToCharacter OtherActor))
  (Variables|Default|SetChar%20REF _ascharacter)
  (bind _returnvalue (Utilities|Time|SetTimerbyEvent (delegate Custom|Rotate) 0.01 true))
  (Variables|Default|SetTimer%20Handle _returnvalue))

(event OnComponentBeginOverlap(Box)
  (params (OverlappedComponent :type Primitive%20Component%20Object%20Reference) (OtherActor :type Actor%20Object%20Reference) (OtherComp :type Primitive%20Component%20Object%20Reference) (OtherBodyIndex :type Integer) (bFromSweep :type Boolean) (SweepResult :type Hit%20Result%20Structure%20%28by%20ref%29))
  (Physics|SetSimulatePhysics (Variables|Default|GetBody) true))

(event Custom|Rotate
  (bind _body (Variables|Default|GetBody))
  (bind _returnvalue (Components|GetOwner _body))
  (Transformation|SetActorRotation _returnvalue (Math|Rotator|MakeRotator 0.0 0.0 (.yaw (Math|Interpolation|RInterpTo (Transformation|GetActorRotation _returnvalue) (Math|Rotator|FindLookatRotation (Transformation|GetActorLocation) (Transformation|GetActorLocation (Variables|Default|GetChar%20REF))) (Utilities|Time|GetWorldDeltaSeconds) 1.0)))))

(event Custom|OnComponentEndOverlap_Event
  (params (OverlappedComponent :type Primitive%20Component%20Object%20Reference) (OtherActor :type Actor%20Object%20Reference) (OtherComp :type Primitive%20Component%20Object%20Reference) (OtherBodyIndex :type Integer))
  (Utilities|Time|ClearandInvalidateTimerbyHandle (Variables|Default|GetTimer%20Handle)))

(event EventBeginPlay)

(event Collision|EventActorBeginOverlap
  (params (OtherActor :type Actor%20Object%20Reference)))

(event EventTick
  (params (DeltaSeconds :type Float%20%28single-precision%29)))

(fn ConstructionScript)